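; CrippledLamp_BP is an enemy actor, a crippled lamp that moves forward in bursts driven by its animation.
; On BeginPlay it caches the CrippledLamp mesh's CrippledLampAnim instance.
; While that instance's OnMove flag is set, each Tick offsets the actor along its forward vector by MoveDistance divided by MoveFrames.
; The step is unswept and ignores delta time, so speed depends on frame rate.
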(event `self.ReceiveBeginPlay`
  (bind _ascrippled_lamp_anim (cast `/Game/Blueprints/Animation/CrippledLamp/CrippledLampAnim` (`SkeletalMeshComponent.GetAnimInstance` (`self.CrippledLamp`))))
  (set `self.CrippledLampAnim` _ascrippled_lamp_anim))

(event `self.ReceiveTick`
  (params (DeltaSeconds :type "Float (single-precision)"))
  (if (`/Game/Blueprints/Animation/CrippledLamp/CrippledLampAnim.OnMove` (`self.CrippledLampAnim`))
    (`self.K2_AddActorWorldOffset` (* (`self.GetActorForwardVector`) (/ (`self.MoveDistance`) (`self.MoveFrames`))))))

(fn `UserConstructionScript`)