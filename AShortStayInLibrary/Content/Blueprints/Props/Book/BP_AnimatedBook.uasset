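; Animated book prop Blueprint that opens and closes a frame mesh and five skeletal page meshes on open and close events.
; It caches their anim instances on BeginPlay, then sets intent and speed variables on them.
; An accumulating timer gives each page a staggered delay, with lag values adjusting page speed and delaying the frame's close.
; On open, it binds to frame anim notifies and re-broadcasts them as its own opened/closed dispatchers.
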(event `OpenBookEvent`
  (bind _bookopenclosespeed (`self.BookOpenCloseSpeed`))
  (bind _pagetimer (`self.PageTimer`))
  (bind _asbook_frame_anim (cast `/Game/Blueprints/Animation/Book/BookFrameAnim` (`SkeletalMeshComponent.GetAnimInstance` (`self.BookFrame`))))
  (add `/Game/Blueprints/Animation/Book/BookFrameAnim.OnBookOpenedNotify` _asbook_frame_anim (delegate `BookOpenedEvent`))
  (add `/Game/Blueprints/Animation/Book/BookFrameAnim.OnBookClosedNotify` _asbook_frame_anim (delegate `BookClosedEvent`))
  (set `/Game/Blueprints/Animation/Book/BookFrameAnim.OnOpenIntention` true (stale `self.ReceiveBeginPlay` _asbook_frame_anim))
  (set `/Game/Blueprints/Animation/Book/BookFrameAnim.BookOpenCloseSpeed` (`self.BookOpenCloseSpeed`) (stale `self.ReceiveBeginPlay` _asbook_frame_anim))
  (`KismetSystemLibrary.PrintString` "Opening Book !")
  ;[1 1 1] Pages open to the right
  (set `self.PageTimer` (`self.OpenFlipInterval`))
  (for _array_element (stale `self.ReceiveBeginPlay` _output_get)
    (set `/Game/Blueprints/Animation/Book/PageBookAnim.PageTurnSpeed` (`self.PageTurnSpeed`) _array_element)
    (set `/Game/Blueprints/Animation/Book/PageBookAnim.BookOpenSpeed` (- _bookopenclosespeed (`KismetMathLibrary.FMin` (`self.OnOpenLag`) _bookopenclosespeed)) _array_element)
    (set `/Game/Blueprints/Animation/Book/PageBookAnim.OnOpen` true _array_element)
    (set `/Game/Blueprints/Animation/Book/PageBookAnim.BookOpenDelay` _pagetimer _array_element)
    (set `self.PageTimer` (+ _pagetimer (`self.OpenFlipInterval`)))))

(event `BookOpenedEvent`
  (`self.OnBookOpenedNotify`))

(event `BookClosedEvent`
  (`self.OnBookClosedNotify`))

(event `CloseBookEvent`
  (bind _bookopenclosespeed (`self.BookOpenCloseSpeed`))
  (bind _pagetimer (`self.PageTimer`))
  (set `self.PageTimer` 0.0)
  (for _array_element (`self.PagesAnim`)
    (set `/Game/Blueprints/Animation/Book/PageBookAnim.BookCloseSpeed` (+ _bookopenclosespeed (`KismetMathLibrary.FMin` (`self.OnCloseLag`) _bookopenclosespeed)) _array_element)
    (set `/Game/Blueprints/Animation/Book/PageBookAnim.OnBookCloseIntention` true _array_element)
    (set `/Game/Blueprints/Animation/Book/PageBookAnim.BookOpenDelay` _pagetimer _array_element)
    (set `self.PageTimer` (+ _pagetimer (`self.CloseFlipInterval`)))
    (`KismetSystemLibrary.Delay` (`self.OnCloseLag`))
    (set `/Game/Blueprints/Animation/Book/BookFrameAnim.OnOpenIntention` false (stale `self.ReceiveBeginPlay` _asbook_frame_anim))
    (`KismetSystemLibrary.PrintString` "Closing Book !")))

(event `self.ReceiveBeginPlay`
  (bind _bookpage_04 (`self.BookPage_04`))
  (bind _bookpage_01 (`self.BookPage_01`))
  (bind _bookpage_05 (`self.BookPage_05`))
  (bind _bookpage_02 (`self.BookPage_02`))
  (bind _bookpage_03 (`self.BookPage_03`))
  (bind _bookframe (`self.BookFrame`))
  (set `self.BookSkeletalMesh` _bookframe)
  (bind _asbook_frame_anim (cast `/Game/Blueprints/Animation/Book/BookFrameAnim` (`SkeletalMeshComponent.GetAnimInstance` _bookframe)))
  ;[1 1 1] Pages open to the right
  (bind _aspage_book_anim (cast `/Game/Blueprints/Animation/Book/PageBookAnim` (`SkeletalMeshComponent.GetAnimInstance` _bookpage_01)))
  (bind _aspage_book_anim_2 (cast `/Game/Blueprints/Animation/Book/PageBookAnim` (`SkeletalMeshComponent.GetAnimInstance` _bookpage_02)))
  (bind _aspage_book_anim_3 (cast `/Game/Blueprints/Animation/Book/PageBookAnim` (`SkeletalMeshComponent.GetAnimInstance` _bookpage_03)))
  (bind _aspage_book_anim_4 (cast `/Game/Blueprints/Animation/Book/PageBookAnim` (`SkeletalMeshComponent.GetAnimInstance` _bookpage_04)))
  (bind _aspage_book_anim_5 (cast `/Game/Blueprints/Animation/Book/PageBookAnim` (`SkeletalMeshComponent.GetAnimInstance` _bookpage_05)))
  (set `self.PagesMeshComponent` (`|MakeArray` _bookpage_01 _bookpage_02 _bookpage_03 _bookpage_04 _bookpage_05))
  (bind _output_get (set `self.PagesAnim` (`|MakeArray` _aspage_book_anim _aspage_book_anim_2 _aspage_book_anim_3 _aspage_book_anim_4 _aspage_book_anim_5))))

(fn `GetPageByIndex`
  (params (PageIndex :type Integer))
  (returns (PageSkeletalMesh :type "SkeletalMeshComponent Object Reference"))
  (return (`|GetArrayItem` (`self.PagesMeshComponent`) PageIndex)))

(fn `UserConstructionScript`)