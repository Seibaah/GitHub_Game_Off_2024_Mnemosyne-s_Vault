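; Test variant of the main player character that feeds aim rotation to its animation instance and handles reading interactable books.
; Overlap events track the current book; E opens it, blends the view to it, shows the cursor and sets the reading state, while P reverses this.
; Timelines fade the player via a material parameter collection, swapping to a see-through material while reading, with a flag blocking input mid-transition.
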(event `self.ReceiveTick`
  (params (DeltaSeconds :type "Float (single-precision)"))
  (bind _playeranim (`self.PlayerAnim`))
  (if (`KismetSystemLibrary.IsValid` _playeranim)
    (set `/Game/Blueprints/Animation/MainCharacter/PlayerAnim.AimRotation` (`KismetMathLibrary.MakeRotFromY` (* (`KismetMathLibrary.BreakRotIntoAxes` (`self.GetControlRotation`)) (-1.0 -1.0 -1.0))) _playeranim)))

(event `self.ReceiveBeginPlay`
  (bind _asplayer_animation_controller (cast `PlayerAnimationController` (`SkeletalMeshComponent.GetAnimInstance` (`self.Mesh`))))
  (bind _output_get (set `self.AnimController` _asplayer_animation_controller))
  (bind _asplayer_anim (cast `/Game/Blueprints/Animation/MainCharacter/PlayerAnim` _output_get))
  (set `self.PlayerAnim` _asplayer_anim))

(event `self.ReceiveActorBeginOverlap`
  (params (OtherActor :type "Actor Object Reference"))
  (bind _asbp_interactable_book (cast `/Game/Blueprints/Props/Book/BP_InteractableBook` OtherActor))
  (if (`KismetSystemLibrary.IsValid` _asbp_interactable_book)
    (set `self.InteractedBook` _asbp_interactable_book)
    (else
      (`KismetSystemLibrary.PrintString` "Failed retrieving book reference"))))

(event `self.ReceiveActorEndOverlap`
  (params (OtherActor :type "Actor Object Reference"))
  (bind _asbp_interactable_book (cast `/Game/Blueprints/Props/Book/BP_InteractableBook` OtherActor))
  (if (`KismetSystemLibrary.IsValid` _asbp_interactable_book)
    (set `self.InteractedBook` null)
    (else
      (`KismetSystemLibrary.PrintString` "Failed retrieving book reference"))))

(event `Key|E`
  (params (Key :type "Key Structure"))
  (bind _interactedbook (`self.InteractedBook`))
  (:`Pressed`
    (if (`KismetSystemLibrary.IsValid` _interactedbook)
      (if (and (`self.InteractTransitionFinished`) (not (`/Game/Blueprints/Props/Book/BP_InteractableBook.OnDestroyWait` _interactedbook)) (not (`/Game/Blueprints/Props/Book/BP_InteractableBook.IsOpened` _interactedbook)))
        (`self.On Interact Start`)
        (`PrimitiveComponent.SetMaterial` (`self.Mesh`) 0 "/Game/3D_Assets/MainCharacter/MCMatSeeThroughMI.MCMatSeeThroughMI")
        (bind (_direction _opacity) (`Timeline|PlayerFadeOutTimeline` :!via `PlayFromStart`)
          (:`Update`
            (`KismetMaterialLibrary.SetScalarParameterValue` "/Game/Materials/PlayerParamCollection.PlayerParamCollection" "PlayerOpacity" _opacity))
          (:`Finished`
            (set `self.InteractTransitionFinished` true)))))))

(event `Key|P` :paused true
  (params (Key :type "Key Structure"))
  (:`Pressed`
    (if (`self.InteractTransitionFinished`)
      (`self.OnInteractStop`)
      (bind (_direction _opacity) (`Timeline|PlayerFadeInTimeline` :!via `PlayFromStart`)
        (:`Update`
          (`KismetMaterialLibrary.SetScalarParameterValue` "/Game/Materials/PlayerParamCollection.PlayerParamCollection" "PlayerOpacity" _opacity))
        (:`Finished`
          (`PrimitiveComponent.SetMaterial` (`self.Mesh`) 0 "/Game/3D_Assets/MainCharacter/MCMat.MCMat")
          (set `self.InteractTransitionFinished` true))))))

(fn `GetPlayerHead`
  (returns (NewParam :type "SceneComponent Object Reference"))
  (return (`self.PlayerHead`)))

(fn `On Interact Start`
  (bind _returnvalue (`GameplayStatics.GetPlayerController` 0))
  (bind _interactedbook (`self.InteractedBook`))
  (set `/Game/Blueprints/Props/Book/BP_InteractableBook.IsOpened` true _interactedbook)
  (set `self.InteractTransitionFinished` false)
  (`/Game/Blueprints/Props/Book/BP_InteractableBook.OpenBook` _interactedbook)
  (`WidgetBlueprintLibrary.SetInputMode_GameAndUIEx` _returnvalue null "DoNotLock" false)
  (set `PlayerController.bShowMouseCursor` true _returnvalue)
  (`PlayerController.SetViewTargetWithBlend` _returnvalue _interactedbook 1.0 "VTBlend_Linear" 0.0 false)
  (`self.SetIsReading` true))

(fn `OnInteractStop`
  (locals (IsBookOpen :type Boolean) (OpenBookTranstionTime :type "Float (double-precision)" :default 1.0))
  (bind _returnvalue (`GameplayStatics.GetPlayerController` 0))
  (bind _interactedbook (`self.InteractedBook`))
  (if (`KismetSystemLibrary.IsValid` _interactedbook)
    ;[1 1 1] Temporary
    (set `self.InteractTransitionFinished` false)
    (`/Game/Blueprints/Props/Book/BP_InteractableBook.Close Book` _interactedbook)
    (`WidgetBlueprintLibrary.SetInputMode_GameOnly` _returnvalue)
    (set `PlayerController.bShowMouseCursor` false _returnvalue)
    (`PlayerController.SetViewTargetWithBlend` _returnvalue (`ActorComponent.GetOwner` (`self.PlayerCameraController`)) 1.0 "VTBlend_Linear" 0.0 false)
    (`self.SetIsReading` false)
    (`self.SetIsReading` false)))

(fn `UserConstructionScript`)