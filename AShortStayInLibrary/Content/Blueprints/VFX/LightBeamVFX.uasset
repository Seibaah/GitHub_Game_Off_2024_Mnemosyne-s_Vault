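; Light beam VFX actor that plays a summon-triggered beam burst between a cone mesh and an end point.
; Two Niagara ring systems follow child-actor splines, with beam parameters and fixed bounds set from the endpoints.
; The summon's fire event triggers, after a delay, a timeline driving cone scale and material collection glow and opacity.
; Mid-burst, it fires the backend event and briefly pulses particle repel force, then applies drag and curl noise.
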(event `self.ReceiveBeginPlay`
  (bind _returnvalue (`SceneComponent.K2_GetComponentLocation` (`self.BeamEnd`)))
  (bind _returnvalue_2 (`SceneComponent.K2_GetComponentLocation` (`self.pewpewCone`)))
  (add `self.BeamFiredVisual` (delegate `BeamStartedEvent`))
  (`self.Bind Niagara Splines`)
  (`self.Niagara Set Beam Properties`)
  (bind _asanimated_summon_bp (cast `/Game/Blueprints/VFX/AnimatedSummon_BP` (`ChildActorComponent.ChildActor` (`self.AnimatedSummon_BP`))))
  (bind _output_get (set `self.AnimatedSummonBP` _asanimated_summon_bp))
  (`/Game/Blueprints/VFX/AnimatedSummon_BP.SetActivationSpeedValue` _output_get (`self.ActivationSpeed`))
  (add `/Game/Blueprints/VFX/AnimatedSummon_BP.FireBeam` _output_get (delegate `FireBeamVFX`))
  (set `self.BeamLength` (`KismetMathLibrary.VSize` (- _returnvalue _returnvalue_2)))
  (set `self.StartPos` _returnvalue_2)
  (set `self.EndPos` _returnvalue))

(event `FireBeamVFX`
  (`KismetSystemLibrary.Delay` (`self.FireDelay`))
  (`self.BeamFiredVisual`))

(event `BeamStartedEvent`
  (bind _relativescale3d_x (`KismetMathLibrary.BreakVector` (`SceneComponent.RelativeScale3D` (`self.pewpewCone`))))
  (`self.Enable VFX`)
  (bind (_direction _scaleinterp _luminosityinterp _beamcoreopacityinterp _time) (`Timeline|BeamBurstTimeline` :!via `PlayFromStart`)
    (:`Update`
      (bind (_returnvalue_x _returnvalue_y _returnvalue_z) (`KismetMathLibrary.BreakVector` (`KismetMathLibrary.MakeVector` 0.0 _scaleinterp _scaleinterp)))
      (`SceneComponent.SetRelativeScale3D` (`self.pewpewCone`) (`KismetMathLibrary.MakeVector` _relativescale3d_x _returnvalue_y _returnvalue_z))
      (`KismetMaterialLibrary.SetScalarParameterValue` "/Game/Materials/LightVFX_MParam_Collection.LightVFX_MParam_Collection" "BeamCoreLumen" _luminosityinterp)
      (`KismetMaterialLibrary.SetScalarParameterValue` "/Game/Materials/LightVFX_MParam_Collection.LightVFX_MParam_Collection" "BeamCoreOpacity" _beamcoreopacityinterp)
      (`/Engine/EditorBlueprintResources/StandardMacros.CompareFloat` _time 0.4
        (:`>`
          (if (not (`self.ForceFieldActivated`))
            (`self.Activate Force Field`)
            (set `self.ForceFieldActivated` true)
            (`self.BeamFiredBackend`)
            (`KismetSystemLibrary.Delay` 0.2)
            (`self.DeactivateForceField`)))))))

(fn `Activate Force Field`
  (bind _returnvalue (* (`self.OutburstStrength`) -1.0))
  (`NiagaraComponent.SetVariableFloat` (`self.BeamRingVFX_2`) "RepelForce" _returnvalue)
  (`NiagaraComponent.SetVariableFloat` (`self.BeamRingVFX_1`) "RepelForce" _returnvalue))

(fn `Bind Niagara Splines`
  (bind _aslight_beam_spline (cast `/Game/Blueprints/VFX/LightBeamSpline` (`ChildActorComponent.ChildActor` (`self.Spline_01`))))
  (`NiagaraComponent.SetVariableObject` (`self.BeamRingVFX_1`) "SplineObject" (`/Game/Blueprints/VFX/LightBeamSpline.SplinePath` _aslight_beam_spline))
  (bind _aslight_beam_spline_2 (cast `/Game/Blueprints/VFX/LightBeamSpline` (`ChildActorComponent.ChildActor` (`self.Spline_02`))))
  (`NiagaraComponent.SetVariableObject` (`self.BeamRingVFX_2`) "SplineObject" (`/Game/Blueprints/VFX/LightBeamSpline.SplinePath` _aslight_beam_spline_2))
  (return))

(fn `DeactivateForceField`
  (bind _beamringvfx_2 (`self.BeamRingVFX_2`))
  (bind _beamringvfx_1 (`self.BeamRingVFX_1`))
  (bind _outburstdrag (`self.OutburstDrag`))
  (bind _returnvalue (/ (`self.OutburstStrength`) (`self.OutburstDrag`)))
  (`NiagaraComponent.SetVariableFloat` _beamringvfx_2 "RepelForce" 0.0)
  (`NiagaraComponent.SetVariableFloat` _beamringvfx_1 "RepelForce" 0.0)
  (`NiagaraComponent.SetVariableFloat` _beamringvfx_2 "Drag" _outburstdrag)
  (`NiagaraComponent.SetVariableFloat` _beamringvfx_1 "Drag" _outburstdrag)
  (`NiagaraComponent.SetVariableFloat` _beamringvfx_2 "CurlNoiseStrength" _returnvalue)
  (`NiagaraComponent.SetVariableFloat` _beamringvfx_1 "CurlNoiseStrength" _returnvalue))

(fn `Disable VFX`
  (`ActorComponent.Deactivate` (`self.BeamRingVFX_1`))
  (`ActorComponent.Deactivate` (`self.BeamRingVFX_2`)))

(fn `Enable VFX`
  (`ActorComponent.Activate` (`self.BeamRingVFX_1`) false)
  (`ActorComponent.Activate` (`self.BeamRingVFX_2`) false))

(fn `Niagara Set Beam Properties`
  (bind _beamringvfx_1 (`self.BeamRingVFX_1`))
  (bind (_beamextents_x _beamextents_y) (`KismetMathLibrary.BreakVector2D` (`self.BeamExtents`)))
  (bind _beamringvfx_2 (`self.BeamRingVFX_2`))
  (bind _beamspeed (`self.BeamSpeed`))
  (bind _beamringvfx_1_2 (`self.BeamRingVFX_1`))
  (bind _returnvalue (`SceneComponent.K2_GetComponentLocation` (`self.pewpewCone`)))
  (bind _returnvalue_2 (`SceneComponent.K2_GetComponentLocation` (`self.BeamEnd`)))
  (bind (_returnvalue_x _returnvalue_y) (`KismetMathLibrary.BreakVector2D` (* (`self.BeamExtents`) (-1.0 -1.0))))
  (bind _returnvalue_3 (`KismetMathLibrary.MakeBox` (`KismetMathLibrary.MakeVector` 0.0 _returnvalue_x _returnvalue_y) (`KismetMathLibrary.MakeVector` (`KismetMathLibrary.VSize` (- (`SceneComponent.K2_GetComponentLocation` (`self.pewpewCone`)) (`SceneComponent.K2_GetComponentLocation` (`self.BeamEnd`)))) _beamextents_x _beamextents_y)))
  (`NiagaraComponent.SetVariableFloat` _beamringvfx_2 "BeamWidth" (`self.BeamRingWidth`))
  (`NiagaraComponent.SetVariableFloat` _beamringvfx_2 "BeamSpeed" _beamspeed)
  (`NiagaraComponent.SetVariableVec3` _beamringvfx_2 "LazerPositionStart" _returnvalue)
  (`NiagaraComponent.SetVariableVec3` _beamringvfx_2 "LazerPositionEnd" _returnvalue_2)
  (`NiagaraComponent.SetVariableFloat` _beamringvfx_1_2 "BeamWidth" (`self.BeamRingWidth`))
  (`NiagaraComponent.SetVariableFloat` _beamringvfx_1_2 "BeamSpeed" _beamspeed)
  (`NiagaraComponent.SetVariableVec3` _beamringvfx_1_2 "LazerPositionStart" _returnvalue)
  (`NiagaraComponent.SetVariableVec3` _beamringvfx_1_2 "LazerPositionEnd" _returnvalue_2)
  (`self.Disable VFX`)
  (`NiagaraComponent.SetSystemFixedBounds` _beamringvfx_1 _returnvalue_3)
  (`NiagaraComponent.SetSystemFixedBounds` _beamringvfx_1 _returnvalue_3)
  (`NiagaraComponent.SetSystemFixedBounds` (`self.BeamRingVFX_2`) _returnvalue_3))

(fn `UserConstructionScript`
  (`self.Bind Niagara Splines`)
  (`self.Niagara Set Beam Properties`))