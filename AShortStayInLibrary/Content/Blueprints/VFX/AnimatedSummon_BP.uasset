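; Summon effect Blueprint that drives an animated summoning-circle mesh and its fire beam through the SummonBeamAnim instance.
; BeginPlay caches that anim instance, binds to its beam-disappear event and sets SummonCircles true, marked as testing.
; The event calls CallFireBeam and plays a timeline feeding dissipation and luminosity into a Material Parameter Collection.
; SetActivationSpeedValue forwards summon speed to the anim instance.
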(event `self.ReceiveBeginPlay`
  (bind _assummon_beam_anim (cast `/Game/Blueprints/Animation/SummonBeam/SummonBeamAnim` (`SkeletalMeshComponent.GetAnimInstance` (`self.plane4pewpew_noscale`)))
    (:`then`
      (bind _output_get (set `self.SummonAnimObject` _assummon_beam_anim))
      (bind _output_get_2 (set `self.SummonAnimObject` _output_get))
      (add `/Game/Blueprints/Animation/SummonBeam/SummonBeamAnim.OnFireBeamDissapear` _output_get_2 (delegate `OnFireBeamEvent`))
      ;[1 1 1] THIS IS FOR TESTING DON'T TOUCH THAT SHIT
      (set `/Game/Blueprints/Animation/SummonBeam/SummonBeamAnim.SummonCircles` true (`self.SummonAnimObject`)))
    (:`CastFailed`
      (`KismetSystemLibrary.PrintString` "CAST FAILED"))))

(event `OnFireBeamEvent`
  (`self.FireBeam`)
  (bind (_direction _dissipatevalue _luminosity) (`Timeline|SummonTimeline`)
    (:`Update`
      (`KismetMaterialLibrary.SetScalarParameterValue` "/Game/Materials/LightVFX_MParam_Collection.LightVFX_MParam_Collection" "SummonDissipate" _dissipatevalue)
      (`KismetMaterialLibrary.SetScalarParameterValue` "/Game/Materials/LightVFX_MParam_Collection.LightVFX_MParam_Collection" "SummonLumen" _luminosity))))

(fn `SetActivationSpeedValue`
  (params (ActivationSpeed :type "Float (double-precision)"))
  (`/Game/Blueprints/Animation/SummonBeam/SummonBeamAnim.SetSummonSpeedValue` (`self.SummonAnimObject`) ActivationSpeed))

(fn `UserConstructionScript`)