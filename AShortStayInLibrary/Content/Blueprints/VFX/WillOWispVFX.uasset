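; WillOWispVFX is a Blueprint wrapper for a will-o'-wisp Niagara effect.
; Its construction script calls InitializeNiagaraParameters, which pushes user parameters into the WillOWispFX component.
; A single SystemScale multiplier derives the core, ember and fire sprite sizes, while two offset vectors position the core and ember source.
; The event graph holds only disabled stub events, so it has no runtime logic.
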(fn `Initialize Niagara Parameters`
  (bind _willowispfx (`self.WillOWispFX`))
  (bind _systemscale (`self.SystemScale`))
  (bind _systemscale_2 (`self.SystemScale`))
  (bind _willowispfx_2 (`self.WillOWispFX`))
  (`NiagaraComponent.SetVariableFloat` _willowispfx_2 "CoreSize" (* _systemscale_2 5.0))
  (`NiagaraComponent.SetVariableFloat` _willowispfx_2 "EmberSize_1" (* _systemscale_2 0.5))
  (`NiagaraComponent.SetVariableFloat` _willowispfx_2 "EmberSize_2" _systemscale)
  (`NiagaraComponent.SetVariableFloat` _willowispfx "FireSpriteSize_1" (* _systemscale 10.0))
  (`NiagaraComponent.SetVariableFloat` _willowispfx "FireSpriteSize_2" (* _systemscale 20.0))
  (`NiagaraComponent.SetVariableVec3` _willowispfx "CorePositionOffset" (`self.CorePositionOffset`))
  (`NiagaraComponent.SetVariableVec3` _willowispfx "EmberSourceOffset" (`self.EmberSourceOffset`)))

(fn `UserConstructionScript`
  (`self.Initialize Niagara Parameters`))