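; Short-lived VFX actor for a light-themed base attack burst that destroys itself one second after BeginPlay.
; BeginPlay binds and immediately fires the InitAttackBurst dispatcher, which sets the burst thickness and plays a timeline.
; The timeline drives the cone cylinder's X/Y scale, keeping Z, and writes fade, opacity and lumen to LightVFX_MParam_Collection.
; Those material values are collection-wide rather than per instance.
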(event `self.ReceiveBeginPlay`
  (add `self.InitAttackBurst` (delegate `OnAttackBurst`))
  (`self.FireAttack`)
  (`KismetSystemLibrary.Delay` 1.0)
  (`self.K2_DestroyActor`))

(event `OnAttackBurst`
  (bind _baseattackcone_cylinder (`self.BaseAttackCone_Cylinder`))
  (bind (_relativescale3d_x _relativescale3d_y _relativescale3d_z) (`KismetMathLibrary.BreakVector` (`SceneComponent.RelativeScale3D` _baseattackcone_cylinder)))
  (`KismetMaterialLibrary.SetScalarParameterValue` "/Game/Materials/LightVFX_MParam_Collection.LightVFX_MParam_Collection" "BaseAttackBurstThickness" 0.1)
  (bind (_direction _burstalpha _baseattackopacity _baseattacklumen _baseattackscale) (`Timeline|Timeline`)
    (:`Update`
      (bind (_returnvalue_x _returnvalue_y) (`KismetMathLibrary.BreakVector` (`KismetMathLibrary.MakeVector` _baseattackscale _baseattackscale)))
      (`SceneComponent.SetRelativeScale3D` _baseattackcone_cylinder (`KismetMathLibrary.MakeVector` _returnvalue_x _returnvalue_y _relativescale3d_z))
      (`KismetMaterialLibrary.SetScalarParameterValue` "/Game/Materials/LightVFX_MParam_Collection.LightVFX_MParam_Collection" "BaseAttackBurstFade" _burstalpha)
      (`KismetMaterialLibrary.SetScalarParameterValue` "/Game/Materials/LightVFX_MParam_Collection.LightVFX_MParam_Collection" "BaseAttackOpacity" _baseattackopacity)
      (`KismetMaterialLibrary.SetScalarParameterValue` "/Game/Materials/LightVFX_MParam_Collection.LightVFX_MParam_Collection" "BaseAttackLumen" _baseattacklumen))))

(fn `FireAttack`
  (`self.InitAttackBurst`))

(fn `UserConstructionScript`)