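; Beam VFX manager that links a LightBeamVFX child actor to its own beam setters and delegate.
; On BeginPlay it casts the child actor and passes that actor's beam length, start position and end position to its own setters.
; It also binds to the child's BeamFiredBackend event and relays each firing through CallBeamDelegate.
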(event `self.ReceiveBeginPlay`
  (bind _aslight_beam_vfx (cast `/Game/Blueprints/VFX/LightBeamVFX` (`ChildActorComponent.ChildActor` (`self.LightBeamVFX`))))
  (`self.SetBeamLength` (`/Game/Blueprints/VFX/LightBeamVFX.BeamLength` _aslight_beam_vfx))
  (add `/Game/Blueprints/VFX/LightBeamVFX.BeamFiredBackend` _aslight_beam_vfx (delegate `BeamFiredEvent`))
  (`self.SetStartPosition` (`/Game/Blueprints/VFX/LightBeamVFX.StartPos` _aslight_beam_vfx))
  (`self.SetEndPosition` (`/Game/Blueprints/VFX/LightBeamVFX.EndPos` _aslight_beam_vfx)))

(event `BeamFiredEvent`
  (`self.BeamDelegate`))

(fn `UserConstructionScript`)