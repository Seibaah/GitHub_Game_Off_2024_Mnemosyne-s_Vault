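; Base Blueprint for a physics body that can be blown apart with an impulse.
; The construction script calls Initialize, which turns on physics simulation for PhysicsMesh.
; BlowUp pushes the mesh at ImpulseLocation, in a random direction within a cone around its forward vector, scaled by BlowUpForce.
; The BlowUp call in the event graph is unconnected, so nothing here triggers it.
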(event `self.ReceiveBeginPlay`)

(fn `BlowUp`
  (bind _physicsmesh (`self.PhysicsMesh`))
  (if (`KismetSystemLibrary.IsValid` (`self.PhysicsMesh`))
    (`PrimitiveComponent.AddImpulseAtLocation` _physicsmesh (* (`KismetMathLibrary.RandomUnitVectorInConeInDegrees` (`SceneComponent.GetForwardVector` _physicsmesh) 45.0) (`self.BlowUpForce`)) (`self.ImpulseLocation`) "None")))

(fn `Initialize`
  (bind _physicsmesh (`self.PhysicsMesh`))
  (if (`KismetSystemLibrary.IsValid` _physicsmesh)
    (`PrimitiveComponent.SetSimulatePhysics` _physicsmesh true)))

(fn `UserConstructionScript`
  (`self.Initialize`))