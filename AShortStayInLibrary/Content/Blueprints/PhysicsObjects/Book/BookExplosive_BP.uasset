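; BookExplosive_BP is an explosive book physics object that wraps a BookRandomMovable_BP child actor.
; Its Initialize function casts the child actor and sets PhysicsMesh to that book's DynamicMesh.
; Initialize runs in both the construction script and BeginPlay, ahead of the parent's logic, so the inherited behavior works on the book's mesh.
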(event `self.ReceiveBeginPlay`
  (`self.Initialize`)
  (`parent.ReceiveBeginPlay`))

(fn `Initialize`
  (bind _asbook_random_movable_bp (cast `/Game/Blueprints/Props/Book/BookRandomMovable_BP` (`ChildActorComponent.ChildActor` (`self.BookRandomMovable_BP`))))
  (set `self.PhysicsMesh` (`/Game/Blueprints/Props/Book/BookRandomMovable_BP.DynamicMesh` _asbook_random_movable_bp)))

(fn `UserConstructionScript`
  (`self.Initialize`)
  (`parent.UserConstructionScript`))